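; Patient actor (remy) for a nursing game that turns and moves in response to boolean flags, none of which it sets to true itself.
; Tick passes the flags to four helper functions.
; Left and right rotations apply a one-shot 90-degree world rotation, then clear their flags.
; Up and down apply small fixed per-frame offsets while flagged, independent of delta time and without sweep; upward movement also drifts along negative X.
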(event `self.ReceiveBeginPlay`
  (set `self.goingUp` false)
  (set `self.goingDown` false))

(event `self.ReceiveTick`
  (params (DeltaSeconds :type "Float (single-precision)"))
  (`self.RotateRightIfCondition` (`self.rotateRight`))
  (`self.RotateLeftIfCondition` (`self.rotateLeft`))
  (`self.GoUpIfCondition` (`self.goingUp`))
  (`self.goDownIfCondition` (`self.goingDown`)))

(fn `goDownIfCondition`
  (params (Condition :type Boolean))
  (if Condition
    (`self.K2_AddActorWorldOffset` (0.0 0.0 -0.3))
    (return)
    (else
      (return))))

(fn `GoUpIfCondition`
  (params (Condition :type Boolean))
  (if Condition
    (`self.K2_AddActorWorldOffset` (-0.1 0.0 0.3))
    (return)
    (else
      (return))))

(fn `RotateLeftIfCondition`
  (params (Condition :type Boolean))
  (if Condition
    (`self.K2_AddActorWorldRotation` (struct :`Yaw` -90.0))
    (set `self.turnLeft` false)
    (set `self.rotateLeft` false)
    (return)
    (else
      (return))))

(fn `RotateRightIfCondition`
  (params (Condition :type Boolean))
  (if Condition
    (`self.K2_AddActorWorldRotation` (struct :`Yaw` 90.0))
    (set `self.turnRight` false)
    (set `self.rotateRight` false)
    (return)
    (else
      (return))))

(fn `UserConstructionScript`)