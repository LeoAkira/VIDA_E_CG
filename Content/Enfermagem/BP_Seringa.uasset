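; BP_Seringa is a syringe for a nursing interaction with Leap Motion hands that appears to draw blood from a vein.
; While its Point overlaps a BP_Veia, Tick lowers the Plunger and stretches and offsets the Blood component to fake filling.
; A Z limit on the Plunger sets MaxLenght to stop the motion.
; Overlaps between the Glass and the Leap hands toggle TocandoDireita (touching right) on the hands character.
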(event `self.ReceiveActorBeginOverlap`
  (params (OtherActor :type "Actor Object Reference")))

(event `self.Point.OnComponentBeginOverlap`
  (params (OverlappedComponent :type "PrimitiveComponent Object Reference") (OtherActor :type "Actor Object Reference") (OtherComp :type "PrimitiveComponent Object Reference") (OtherBodyIndex :type Integer) (bFromSweep :type Boolean) (SweepResult :type "HitResult Structure (by ref)"))
  (if (== (`GameplayStatics.GetObjectClass` OtherActor) "/Game/Enfermagem/BP_Veia.BP_Veia_C")
    (set `self.speed` 0.6)))

(event `self.Point.OnComponentEndOverlap`
  (params (OverlappedComponent :type "PrimitiveComponent Object Reference") (OtherActor :type "Actor Object Reference") (OtherComp :type "PrimitiveComponent Object Reference") (OtherBodyIndex :type Integer))
  (if (== (`GameplayStatics.GetObjectClass` OtherActor) "/Game/Enfermagem/BP_Veia.BP_Veia_C")
    (set `self.speed` 0.0)))

(event `self.ReceiveTick`
  (params (DeltaSeconds :type "Float (single-precision)"))
  (`self.movePlunger` (`self.speed`)))

(event `self.Glass.OnComponentBeginOverlap`
  (params (OverlappedComponent :type "PrimitiveComponent Object Reference") (OtherActor :type "Actor Object Reference") (OtherComp :type "PrimitiveComponent Object Reference") (OtherBodyIndex :type Integer) (bFromSweep :type Boolean) (SweepResult :type "HitResult Structure (by ref)"))
  (if (== (`GameplayStatics.GetObjectClass` OtherActor) "/LeapMotion/Blueprints/Rigging/FloatingHands/LeapRiggedEchoHandsActor.LeapRiggedEchoHandsActor_C")
    (bind _asbp_leap_floating_hands_character (cast `/Game/Enfermagem/BP_LeapFloatingHandsCharacter` (`self.GetParentActor` OtherActor)))
    (set `/Game/Enfermagem/BP_LeapFloatingHandsCharacter.tocandoDireita` true _asbp_leap_floating_hands_character)))

(event `self.Glass.OnComponentEndOverlap`
  (params (OverlappedComponent :type "PrimitiveComponent Object Reference") (OtherActor :type "Actor Object Reference") (OtherComp :type "PrimitiveComponent Object Reference") (OtherBodyIndex :type Integer))
  (if (== (`GameplayStatics.GetObjectClass` OtherActor) "/LeapMotion/Blueprints/Rigging/FloatingHands/LeapRiggedEchoHandsActor.LeapRiggedEchoHandsActor_C")
    (bind _asbp_leap_floating_hands_character (cast `/Game/Enfermagem/BP_LeapFloatingHandsCharacter` (`self.GetParentActor` OtherActor)))
    (set `/Game/Enfermagem/BP_LeapFloatingHandsCharacter.tocandoDireita` false _asbp_leap_floating_hands_character)))

(fn `moveInZ`
  (params (speed :type "Float (double-precision)") (self2 :type "SceneComponent Object Reference"))
  (bind _relativelocation (`SceneComponent.RelativeLocation` self2))
  (`/Engine/EditorBlueprintResources/StandardMacros.CompareFloat` (.z _relativelocation) -275.0
    (:`>`
      (set `self.MaxLenght` false :!label _label))
    (:`==`
      (goto _label))
    (:`<`
      (set `self.MaxLenght` true)))
  (`SceneComponent.K2_SetRelativeLocation` self2 (+ _relativelocation (* (0.0 0.0 -1.0) speed)) false false)
  (return))

(fn `movePlunger`
  (params (speed :type "Float (double-precision)"))
  (if (not (`self.MaxLenght`))
    (`self.scaleAndMoveInZ` speed (`self.Blood`))
    (`self.moveInZ` speed (`self.Plunger`))))

(fn `scaleAndMoveInZ`
  (params (speed :type "Float (double-precision)") (Object :type "SceneComponent Object Reference"))
  (`SceneComponent.SetRelativeScale3D` Object (+ (`SceneComponent.RelativeScale3D` Object) (* (0.0 0.0 0.01) speed)))
  (`SceneComponent.K2_SetRelativeLocation` Object (+ (`SceneComponent.RelativeLocation` Object) (* (0.0 0.0 -0.5) speed)) false false)
  (return))

(fn `UserConstructionScript`)